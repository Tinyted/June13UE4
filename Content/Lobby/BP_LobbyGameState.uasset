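; Lobby GameState that keeps player lists current and sets the default map for the lobby.
; Post-login and refresh notifications loop over PlayerArray, telling each owning BP_LobbyPlayerController to update its list.
; A team-info rep callback, meant for clients, refreshes the first local controller's list immediately to avoid replication latency.
; SetDefaultSelectedMap, called by the GameMode, selects the first available map on the server, warning otherwise.
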(event Custom|NotifyPostLogin
  (for _array_element (Variables|Default|GetPlayerArray)
    (bind _asbp_lobby_player_controller (Utilities|Casting|CastToBP_LobbyPlayerController (Components|GetOwner _array_element))
      (:then
        (Default|UpdatePlayerList _asbp_lobby_player_controller))
      (:CastFailed
        (Development|PrintString "BP: LobbyGameState cast failed for casting BP_LobbyPlayerController")))))

(event Custom|NotifyRefreshPlayerList
  (for _array_element (Variables|Default|GetPlayerArray)
    (bind _asbp_lobby_player_controller (Utilities|Casting|CastToBP_LobbyPlayerController (Components|GetOwner _array_element))
      (:then
        (Default|UpdatePlayerList _asbp_lobby_player_controller))
      (:CastFailed
        (Development|PrintString "BP: LobbyGameState cast failed for casting BP_LobbyPlayerController")))))

(event EventBeginPlay)

(event EventTick
  (params (DeltaSeconds :type Float%20%28single-precision%29)))

(event EventSetDefaultSelectedMap
  (bind _mapsavailable (Variables|Default|GetMapsAvailable))
  ;[1 1 1] Called by GameMode so shouldn't need to check for server
  (Development|PrintString "BP LobbyGameState SetDefaultMap" false)
  (if (> (Utilities|Array|Length _mapsavailable) 0)
    (if (Networking|IsServer)
      (Class|LobbyGameState|ServerSetCurrentSelectedMap (Utilities|Array|Get(acopy) _mapsavailable))
      (else
        (Development|PrintString "WARNING: Client tried to set current selected map")))
    (else
      (Development|PrintString "WARNING: BP_LobbyGameState should start with a default selected map"))))

(event EventOnRepTeamInfoChanged
  ;[1 1 1] Used to avoid latency issues with replication when teaminfo is changed, by having an instant callback to update playlist. Should only be called on nonServers
  (bind _asbp_lobby_player_controller (Utilities|Casting|CastToBP_LobbyPlayerController (Game|GetPlayerController 0)))
  (Default|UpdatePlayerList _asbp_lobby_player_controller))

(fn ConstructionScript)