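; Lobby game mode that handles player logins and starts map travel out of the lobby.
; On PostLogin it calls NotifyPostLogin on BP_LobbyGameState, printing a message if that cast fails.
; Server_MapTravel temporarily sets the game state's selected map to the first available entry, then calls ServerTravel, doing nothing further if no map exists.
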(event Custom|Server_MapTravel
  (Development|PrintString "ServerMapTravel")
  ;[1 1 1] TEMP Set Selected Map and Mode
  (bind _asbp_lobby_game_state (Utilities|Casting|CastToBP_LobbyGameState (Game|GetGameState)))
  (if (Utilities|Array|IsValidIndex (Variables|/Script/June13.LobbyGameState|GetMapsAvailable _asbp_lobby_game_state))
    (Variables|/Script/June13.LobbyGameState|SetCurrentSelectedMap _asbp_lobby_game_state (Utilities|Array|Get(acopy) (Variables|/Script/June13.LobbyGameState|GetMapsAvailable _asbp_lobby_game_state)))
    (Class|LobbyGameMode|ServerTravel)))

(event EventBeginPlay
  (Development|PrintString "BP: LobbyGameMode BeginPlay"))

(event EventTick
  (params (DeltaSeconds :type Float%20%28single-precision%29)))

(event EventPostLogin
  (params (NewPlayer :type Player%20Controller%20Object%20Reference))
  (Development|PrintString "BP: LobbyGameMode onPostLogin")
  (bind _asbp_lobby_game_state (Utilities|Casting|CastToBP_LobbyGameState (Game|GetGameState))
    (:then
      (Default|NotifyPostLogin _asbp_lobby_game_state))
    (:CastFailed
      (Development|PrintString "BP: LobbyGameMode cast Failed for BP_LobbyGameState"))))

(fn ConstructionScript)