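; Lobby player controller that shows the lobby UI and lets the server start the match map travel.
; When playing state begins, used instead of BeginPlay so PlayerState is set, it creates the lobby widget and fills it.
; Update events rebuild the player list from the game state's PlayerArray and the map list from BP_LobbyGameState's MapsAvailable.
; Pressing F on the server calls ServerMapTravel on the lobby game mode.
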(event Custom|UpdatePlayerList
  ;[1 1 1] Update Player List
  (Development|PrintString (Utilities|String|Append "BP_LobbyPlayerController UpdatePlayerList for:" (Variables|/Script/Engine.PlayerState|GetPlayerName (Variables|Default|GetPlayerState))))
  (Utilities|IsValid (Variables|Default|GetWidget%20Reference)
    (:Is%20Valid
      (CallFunction|RemoveAllPlayersfromVerticalBox)
      (for _array_element (Variables|/Script/Engine.GameState|GetPlayerArray (Game|GetGameState))
        (CallFunction|AddPlayerNametoVerticalBox (Variables|/Script/Engine.PlayerState|GetPlayerName _array_element))))))

(event Custom|UpdateMapsAvailable
  ;[1 1 1] UpdateMapsAvailable
  (Utilities|IsValid (Variables|Default|GetWidget%20Reference)
    (:Is%20Valid
      (CallFunction|RemoveAllMapnamesfromVerticalBox)
      (bind _asbp_lobby_game_state (Utilities|Casting|CastToBP_LobbyGameState (Game|GetGameState)))
      (for _array_element (Variables|/Script/June13.LobbyGameState|GetMapsAvailable _asbp_lobby_game_state)
        (CallFunction|AddMapNametoVerticalBox (.MapName (Utilities|Struct|BreakMapInfo _array_element)))))))

(event EventBeginPlay
  (Development|PrintString "BP:LobbyPlayerController BeginPlay"))

(event EventTick
  (params (DeltaSeconds :type Float%20%28single-precision%29))
  ;[1 1 1] Not using BeginPlay as that is for Actors (playerstate isnt set on Actor's BeginPlay)
)

(event EventOnBeginPlayingState
  ;[1 1 1] Not using BeginPlay as that is for Actors (playerstate isnt set on Actor's BeginPlay)
  (Development|PrintString (Utilities|String|Append "BP_LobbyPlayerController BeginPlayer for:" (Variables|/Script/Engine.PlayerState|GetPlayerName (Variables|Default|GetPlayerState))))
  (bind _returnvalue (UserInterface|CreateWidget "/Game/LobbyWidgets/BP_Lobby_Widget.BP_Lobby_Widget_C"))
  (bind _output_get (Variables|Default|SetWidget%20Reference _returnvalue))
  (UserInterface|Viewport|AddtoViewport _output_get 0)
  (Development|PrintString "BP: Added Lobby Widget to View Port")
  (CallFunction|UpdatePlayerList)
  (CallFunction|UpdateMapsAvailable))

(event Input|KeyboardEvents|F
  (params (Key :type Key%20Structure :default "AnyKey"))
  (:Pressed
    (Development|PrintString "F Pressed")
    (if (Networking|IsServer)
      (bind _asbp_lobby_game_mode (Utilities|Casting|CastToBP_LobbyGameMode (Game|GetGameMode))
        (:then
          (Development|PrintString "Going to Server Travel")
          (Default|ServerMapTravel _asbp_lobby_game_mode))
        (:CastFailed
          (Development|PrintString "BP_LobbyPlayerController cast fail for gamemode")))
      (else
        (Development|PrintString "Not Server")))))

(fn ConstructionScript)

(fn AddPlayerNametoVerticalBox
  (params (PlayerName :type String))
  (bind _returnvalue (UserInterface|CreateWidget "/Game/LobbyWidgets/BP_Lobby_PlayerName_Widget.BP_Lobby_PlayerName_Widget_C"))
  (Rendering|Components|TextRender|SetText (Variables|/Game/LobbyWidgets/BP_Lobby_PlayerName_Widget.BP_Lobby_PlayerName_Widget_C|GetPlayerNameText _returnvalue) (Utilities|Text|ToText(String) PlayerName))
  (Class|VerticalBox|AddChildtoVerticalBox (Variables|/Game/LobbyWidgets/BP_Lobby_Widget.BP_Lobby_Widget_C|GetPlayerNameVerticalBox (Variables|Default|GetWidget%20Reference)) _returnvalue))

(fn RemoveAllPlayersfromVerticalBox
  (Widget|Panel|ClearChildren (Variables|/Game/LobbyWidgets/BP_Lobby_Widget.BP_Lobby_Widget_C|GetPlayerNameVerticalBox (Variables|Default|GetWidget%20Reference))))

(fn AddMapNametoVerticalBox
  (params (MapName :type String))
  (Development|PrintString "BP: LobbyPlayerController Add Map Name")
  (bind _returnvalue (UserInterface|CreateWidget "/Game/LobbyWidgets/BP_Lobby_MapName_Widget.BP_Lobby_MapName_Widget_C"))
  (Rendering|Components|TextRender|SetText (Variables|/Game/LobbyWidgets/BP_Lobby_MapName_Widget.BP_Lobby_MapName_Widget_C|GetMapNameText _returnvalue) (Utilities|Text|ToText(String) MapName))
  (Class|VerticalBox|AddChildtoVerticalBox (Variables|/Game/LobbyWidgets/BP_Lobby_Widget.BP_Lobby_Widget_C|GetMapsAvailableVerticalBox (Variables|Default|GetWidget%20Reference)) _returnvalue))

(fn RemoveAllMapnamesfromVerticalBox
  (Widget|Panel|ClearChildren (Variables|/Game/LobbyWidgets/BP_Lobby_Widget.BP_Lobby_Widget_C|GetMapsAvailableVerticalBox (Variables|Default|GetWidget%20Reference))))